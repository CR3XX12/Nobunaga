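; TrollBP is a troll enemy that turns around at InvisibleWall actors and damages the player on contact.
; Capsule overlap with a wall toggles IsFacingLeft and snaps the actor's rotation to match.
; On capsule hit, the player's State decides the outcome: DEFAULT takes damage, while PWUPINVINCIBLE destroys the troll.
; The hit-side check compares the player's Y to itself, so damage always reports HitOnLeft as true.
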(event `self.CapsuleComponent.OnComponentBeginOverlap`
  (params (OverlappedComponent :type "PrimitiveComponent Object Reference") (OtherActor :type "Actor Object Reference") (OtherComp :type "PrimitiveComponent Object Reference") (OtherBodyIndex :type Integer) (bFromSweep :type Boolean) (SweepResult :type "HitResult Structure (by ref)"))
  (cast `/Game/Blueprints/Objects/InvisibleWall` OtherActor)
  (bind _output_get (set `self.IsFacingLeft` (not (`self.IsFacingLeft`))))
  (if _output_get
    (`self.K2_SetActorRotation` (struct))
    (else
      (`self.K2_SetActorRotation` (struct :`Yaw` 180.0)))))

(event `self.CapsuleComponent.OnComponentHit`
  (params (HitComponent :type "PrimitiveComponent Object Reference") (OtherActor :type "Actor Object Reference") (OtherComp :type "PrimitiveComponent Object Reference") (NormalImpulse :type "Vector Structure") (Hit :type "HitResult Structure (by ref)"))
  (bind _asteam_8_final_comp217character (cast `Team8_FinalCOMP217Character` OtherActor))
  (switch `ECharacterState` (`Team8_FinalCOMP217Character.state` _asteam_8_final_comp217character)
    (:`E_Default`
      (bind (_returnvalue_x _returnvalue_y) (`KismetMathLibrary.BreakVector` (`self.K2_GetActorLocation` _asteam_8_final_comp217character)))
      (bind (_returnvalue_x_2 _returnvalue_y_2) (`KismetMathLibrary.BreakVector` (`self.K2_GetActorLocation` _asteam_8_final_comp217character)))
      (if (> _returnvalue_y _returnvalue_y_2)
        (`Team8_FinalCOMP217Character.TakeDamage` _asteam_8_final_comp217character 1 false)
        (else
          (`Team8_FinalCOMP217Character.TakeDamage` _asteam_8_final_comp217character 1 true))))
    (:`E_PwUpPickup_i`
      (`self.K2_DestroyActor`))))

(fn `UserConstructionScript`)